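; BP_PlagueRats is an actor that drives a Niagara rat swarm reacting to actors entering its collision volume.
; Begin overlap stores any overlapping actor as AttackTarget and switches on the User.AttackRange parameter, while any end overlap clears both.
; While a target is valid, Tick feeds player 0's location, rather than the target's, into User.PlayerLocation on the Niagara component.
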(event OnComponentBeginOverlap(CollisionDetection)
  (params (OverlappedComponent :type Primitive%20Component%20Object%20Reference) (OtherActor :type Actor%20Object%20Reference) (OtherComp :type Primitive%20Component%20Object%20Reference) (OtherBodyIndex :type Integer) (bFromSweep :type Boolean) (SweepResult :type Hit%20Result%20Structure%20%28by%20ref%29))
  (Variables|Default|SetAttackTarget OtherActor)
  (Niagara|SetNiagaraVariable(Float) (Variables|Default|GetNiagara_Rats) "User.AttackRange" 1.0))

(event OnComponentEndOverlap(CollisionDetection)
  (params (OverlappedComponent :type Primitive%20Component%20Object%20Reference) (OtherActor :type Actor%20Object%20Reference) (OtherComp :type Primitive%20Component%20Object%20Reference) (OtherBodyIndex :type Integer))
  (Variables|Default|SetAttackTarget 0)
  (Niagara|SetNiagaraVariable(Float) (Variables|Default|GetNiagara_Rats) "User.AttackRange" 0.0))

(event EventTick
  (params (DeltaSeconds :type Float%20%28single-precision%29))
  (Utilities|IsValid (Variables|Default|GetAttackTarget)
    (:Is%20Valid
      (Niagara|SetNiagaraVariable(Vector3) (Variables|Default|GetNiagara_Rats) "User.PlayerLocation" (Transformation|GetActorLocation (Game|GetPlayerCharacter 0))))))

(fn ConstructionScript)